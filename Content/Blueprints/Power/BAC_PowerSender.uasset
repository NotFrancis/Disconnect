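; BAC_PowerSender is an actor component that passes power from its owner to a list of target actors.
; SendPower and RemovePower loop over ActorsToSendTo and call Power or Depower on each one's BAC_PowerComponent, passing the owner as source.
; When BindToPowerComponent is set, BeginPlay binds events to the owner's own BAC_PowerComponent powered and depowered notifications, so power components can be chained.
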(event EventBeginPlay
  (if (Variables|Default|GetBindToPowerComponent)
    (CallFunction|SetupPoweredComponentBindings)))

(fn SendPower
  (for _array_element (Variables|Default|GetActorsToSendTo)
    (Default|Power (Actor|GetComponentbyClass _array_element "/Game/Blueprints/Power/BAC_PowerComponent.BAC_PowerComponent_C") (Components|GetOwner))))

(fn RemovePower
  (for _array_element (Variables|Default|GetActorsToSendTo)
    (Default|Depower (Actor|GetComponentbyClass _array_element "/Game/Blueprints/Power/BAC_PowerComponent.BAC_PowerComponent_C") (Components|GetOwner))))

(fn SetupPoweredComponentBindings
  (bind _returnvalue (Components|GetOwner))
  (bind _returnvalue_2 (Actor|GetComponentbyClass _returnvalue "/Game/Blueprints/Power/BAC_PowerComponent.BAC_PowerComponent_C"))
  (EventDispatchers|BindEventtoOnPowered _returnvalue_2 (EventDispatchers|CreateEvent :!event SendPower))
  (EventDispatchers|BindEventtoOnDepowered _returnvalue_2 (EventDispatchers|CreateEvent :!event RemovePower)))