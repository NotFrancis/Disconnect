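; BP_SocketBase is a power socket actor that captures BP_Plug actors entering its box trigger.
; When empty, it notifies the plug of insertion, stores it as the inserted plug, and grabs its component with a Physics Handle.
; The handle's target is set to the PlugSnapPosition transform, so the plug is pulled into place physically.
; RemovePlug releases the handle, notifies the plug and clears the reference, freeing the socket.
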(event OnComponentBeginOverlap(Box)
  (params (OverlappedComponent :type Primitive%20Component%20Object%20Reference) (OtherActor :type Actor%20Object%20Reference) (OtherComp :type Primitive%20Component%20Object%20Reference) (OtherBodyIndex :type Integer) (bFromSweep :type Boolean) (SweepResult :type Hit%20Result%20Structure%20%28by%20ref%29))
  (bind _asbp_plug (Utilities|Casting|CastToBP_Plug OtherActor))
  (CallFunction|InsertPlug _asbp_plug))

(fn ConstructionScript)

(fn InsertPlug
  (params (Plug :type BP%20Plug%20Object%20Reference))
  (bind _plugsnapposition (Variables|Default|GetPlugSnapPosition))
  (bind _returnvalue (Transformation|GetWorldTransform _plugsnapposition))
  (bind _returnvalue_2 (Transformation|GetWorldTransform (Variables|/Game/Blueprints/Power/Plugs/BP_Plug.BP_Plug_C|GetPlug Plug)))
  ;[1 1 1] Check oif we don't have a plug already
  (Utilities|IsValid (Variables|Socketing|GetInsertedPlug)
    (:Is%20Not%20Valid
      ;[1 1 1] Set the plug settings
      (Default|OnPlugInsertion Plug self)
      (Variables|Socketing|SetInsertedPlug Plug)
      (Physics|Components|PhysicsHandle|GrabComponentatLocationwithRotation (Variables|Default|GetPhysicsHandle) (Variables|/Game/Blueprints/Power/Plugs/BP_Plug.BP_Plug_C|GetPlug Plug) "None" (.location _returnvalue_2) (.rotation _returnvalue_2))
      (Class|PhysicsHandleComponent|SetTargetLocationandRotation (Variables|Default|GetPhysicsHandle) (.location _returnvalue) (.rotation _returnvalue)))))

(fn RemovePlug
  (Physics|Components|PhysicsHandle|ReleaseComponent (Variables|Default|GetPhysicsHandle))
  (Default|OnPlugRemoval (Variables|Socketing|GetInsertedPlug))
  (Variables|Socketing|SetInsertedPlug 0))