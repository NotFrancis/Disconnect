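; A plug Blueprint for one end of a wired pair, which passes power between the sockets that it and its ConnectedPlug occupy.
; On a power update, if the other end is socketed, each plug powers or depowers its own socket to match the powered state of its sibling's socket.
; When this plug's socket is invalid, it depowers the socket at the other end.
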(event EventBeginPlay)

(event Collision|EventActorBeginOverlap
  (params (OtherActor :type Actor%20Object%20Reference)))

(event EventTick
  (params (DeltaSeconds :type Float%20%28single-precision%29)))

(fn ConstructionScript
  (|CallParentFunction))

(fn UpdatePower
  (params (Socket :type BP%20Socket%20Base%20Object%20Reference))
  (|CallParentFunction Socket)
  ;[1 1 1] Is the other end plugged in?
  (Utilities|IsValid (Variables|/Game/Blueprints/Power/Plugs/BP_Plug.BP_Plug_C|GetMySocket (Variables|Attributes|GetConnectedPlug))
    (:Is%20Valid
      ;[1 1 1] Are both sockets plugged in?
      (Utilities|IsValid Socket
        (:Is%20Valid
          (Power|CheckifSiblingPowered)
          (Power|CheckifSiblingPowered (Variables|Attributes|GetConnectedPlug)))
        (:Is%20Not%20Valid
          (Default|Depower (Variables|/Game/Blueprints/Power/BP_SocketBase.BP_SocketBase_C|GetBAC_PowerComponent (Variables|/Game/Blueprints/Power/Plugs/BP_Plug.BP_Plug_C|GetMySocket (Variables|Attributes|GetConnectedPlug))) self))))))

(fn CheckifSiblingPowered
  (bind _self self)
  (bind _mysocket (Variables|Default|GetMySocket))
  (bind _bac_powercomponent (Variables|/Game/Blueprints/Power/BP_SocketBase.BP_SocketBase_C|GetBAC_PowerComponent _mysocket))
  (if (Variables|/Game/Blueprints/Power/BAC_PowerComponent.BAC_PowerComponent_C|GetPowered (Variables|/Game/Blueprints/Power/BP_SocketBase.BP_SocketBase_C|GetBAC_PowerComponent (Variables|/Game/Blueprints/Power/Plugs/BP_Plug.BP_Plug_C|GetMySocket (Variables|Attributes|GetConnectedPlug))))
    (Default|Power _bac_powercomponent _self)
    (else
      (Default|Depower _bac_powercomponent _self))))