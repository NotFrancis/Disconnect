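; Grabbable, color-coded power plug that fits into sockets, tinted at construction through a dynamic material instance.
; Insertion stores the socket and force-releases the plug from the player's physics handle if held.
; Grabbing a socketed plug asks the socket to remove it; the removal callback depowers that socket's power component and clears the reference.
; UpdatePower only handles depowering; powering up is not done here.
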(event EventGrabActor
  (bind _mysocket (Variables|Components|GetMySocket))
  ;[1 1 1] If we're in a socket; unplug time
  (Utilities|IsValid _mysocket
    (:Is%20Valid
      (Default|RemovePlug _mysocket))))

(fn ConstructionScript
  (Setup|CreateDMI)
  (CallFunction|ChangePlugColor (Variables|Attributes|GetColor)))

(fn ChangePlugColor
  (params (E_Color :type E_PlugColors%20Enum :default "NewEnumerator0"))
  (Rendering|Material|SetVectorParameterValue (Variables|DMI|GetDMI_Plug) "Color" (CallFunction|GetPlugColor E_Color) :!class /Script/Engine.MaterialInstanceDynamic)
  (return))

(fn CreateDMI
  (bind _plug (Variables|Components|GetPlug))
  (bind _returnvalue (Rendering|Material|CreateDynamicMaterialInstance _plug 0 (Rendering|Material|GetMaterial _plug 0) "None" :!class /Script/Engine.PrimitiveComponent))
  (Variables|DMI|SetDMI_Plug _returnvalue))

(fn OnPlugInsertion
  (params (Socket :type BP%20Socket%20Base%20Object%20Reference))
  (bind _output_get (Variables|Components|SetMySocket Socket))
  (Power|UpdatePower _output_get)
  ;[1 1 1] Hacky? Release this plug when we're holding it. Maybe remove this later.
  (bind _asbp_disconnect_first_person_character (Utilities|Casting|CastToBP_DisconnectFirstPersonCharacter (Game|Player|GetPlayerPawn 0)))
  (Utilities|IsValid (Class|PhysicsHandleComponent|GetGrabbedComponent (Variables|/Game/Blueprints/Characters/BP_DisconnectFirstPersonCharacter.BP_DisconnectFirstPersonCharacter_C|GetPhysicsHandle _asbp_disconnect_first_person_character))
    (:Is%20Valid
      (if (== (Components|GetOwner (Class|PhysicsHandleComponent|GetGrabbedComponent (Variables|/Game/Blueprints/Characters/BP_DisconnectFirstPersonCharacter.BP_DisconnectFirstPersonCharacter_C|GetPhysicsHandle _asbp_disconnect_first_person_character))) self)
        (Default|ReleaseObject _asbp_disconnect_first_person_character)))))

(fn OnPlugRemoval
  (Power|UpdatePower)
  (Variables|Components|SetMySocket 0))

(fn UpdatePower
  (params (Socket :type BP%20Socket%20Base%20Object%20Reference))
  ;[1 1 1] Is it plugged in? If no; then socket isn't powered.
  (Utilities|IsValid Socket
    (:Is%20Not%20Valid
      (Default|Depower (Variables|/Game/Blueprints/Power/BP_SocketBase.BP_SocketBase_C|GetBAC_PowerComponent (Variables|Components|GetMySocket)) self))))

(fn CanInteract
  (return true))