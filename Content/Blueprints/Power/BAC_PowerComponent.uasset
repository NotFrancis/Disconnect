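; Actor component that tracks whether its owner is powered, based on a set of registered power sources.
; Power and Depower add or remove unique sources and compare the count against a required threshold, firing OnPowered or OnDepowered only when the state changes.
; A permanently powered component registers its owner as a source on BeginPlay and, once powered, never depowers.
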(event EventBeginPlay
  (if (Variables|Default|GetPermanentlyPowered)
    (CallFunction|Power (Components|GetOwner))))

(fn Power
  (params (PowerSource :type Actor%20Object%20Reference))
  (Utilities|Array|AddUnique (Variables|Default|GetPowerSources) PowerSource)
  (if (and (not (Variables|Default|GetPowered)) (>= (Utilities|Array|Length (Variables|Default|GetPowerSources)) (Variables|Default|GetPowerSourcesRequired)))
    (Variables|Default|SetPowered true)
    (Default|CallOnPowered)))

(fn Depower
  (params (PowerSource :type Actor%20Object%20Reference))
  (Utilities|Array|RemoveItem (Variables|Default|GetPowerSources) PowerSource)
  ;[1 1 1] If we're powered and not permanently powered, we can depower.
  (if (Math|Boolean|ANDBoolean (Variables|Default|GetPowered) (not (Variables|Default|GetPermanentlyPowered)) (< (Utilities|Array|Length (Variables|Default|GetPowerSources)) (Variables|Default|GetPowerSourcesRequired)))
    (Variables|Default|SetPowered false)
    (Default|CallOnDepowered)))